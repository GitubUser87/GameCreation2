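; BP_HealthPickup is a spinning health pickup that restores 20 health to the first-person character, capped at 100.
; A box overlap casts to BP_FirstPersonCharacter, adjusts its Health directly and plays a 2D pickup sound.
; It then hides the mesh and disables box collision, using a Delay to respawn in place after 20 seconds.
; Tick yaws the actor at a frame-rate-independent rate set by Rotation.
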(event `self.ReceiveTick`
  (params (DeltaSeconds :type "Float (single-precision)"))
  ;[1 1 1] Rotate
  (`self.K2_AddActorLocalRotation` (`KismetMathLibrary.MakeRotator` 0.0 0.0 (* (`self.Rotation`) DeltaSeconds))))

(event `self.Box.OnComponentBeginOverlap`
  (params (OverlappedComponent :type "PrimitiveComponent Object Reference") (OtherActor :type "Actor Object Reference") (OtherComp :type "PrimitiveComponent Object Reference") (OtherBodyIndex :type Integer) (bFromSweep :type Boolean) (SweepResult :type "HitResult Structure (by ref)"))
  ;[1 1 1] Pickup
  (bind _asbp_first_person_character (cast `/Game/FirstPerson/Blueprints/BP_FirstPersonCharacter` OtherActor))
  (bind _health (`/Game/FirstPerson/Blueprints/BP_FirstPersonCharacter.Health` _asbp_first_person_character))
  (if (>= _health 80.0)
    (set `/Game/FirstPerson/Blueprints/BP_FirstPersonCharacter.Health` 100.0 _asbp_first_person_character)
    (else
      (set `/Game/FirstPerson/Blueprints/BP_FirstPersonCharacter.Health` (+ _health 20.0) _asbp_first_person_character)))
  (`GameplayStatics.PlaySound2D` "/Engine/VREditor/Sounds/UI/Object_PickUp.Object_PickUp" 1.0 1.0 0.0 null null)
  (`SceneComponent.SetVisibility` (`self.StaticMesh`) false false)
  (`PrimitiveComponent.SetCollisionEnabled` (`self.Box`) "NoCollision")
  (`KismetSystemLibrary.Delay` 20.0)
  (`PrimitiveComponent.SetCollisionEnabled` (`self.Box`) "QueryAndPhysics")
  (`SceneComponent.SetVisibility` (`self.StaticMesh`) true false))

(fn `UserConstructionScript`)