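; BP_Lever is an interactable lever that opens the BP_Door whose DoorValue matches its LeverValue.
; Interact plays a timeline that rotates the handle and, from its update through a delay, searches all doors for that match.
; A match opens the door, disables the lever base's collision and plays a one-time sound.
; A box overlap shows or hides an interact prompt widget for the player.
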(event `/Game/Maps/General_Content/Blueprints/BP_Interact_Interface.Interact`
  ;[1 1 1] Open Door
  (bind (_direction _pull_track) (`Timeline|Timeline`)
    (:`Update`
      (`SceneComponent.K2_SetRelativeRotation` (`self.Handle`) (`KismetMathLibrary.RLerp` (`self.Current Rotation`) (`self.New Rotation`) _pull_track) false false)
      (`KismetSystemLibrary.Delay` 0.5)
      (bind _outactors (`GameplayStatics.GetAllActorsOfClass` "/Game/Maps/General_Content/Blueprints/BP_Door.BP_Door_C"))
      (for _array_element _outactors
        (if (== (`/Game/Maps/General_Content/Blueprints/BP_Door.Door_Value` _array_element) (`self.Lever_Value`))
          (`/Game/Maps/General_Content/Blueprints/BP_Door.Door Open` _array_element)
          (`|ExecutionSequence`
            (:`then_0`
              (`PrimitiveComponent.SetCollisionEnabled` (`self.Base`) "NoCollision")
              (break))
            (:`then_1`
              (`/Engine/EditorBlueprintResources/StandardMacros.DoOnce` false
                (:`Completed`
                  (`GameplayStatics.PlaySound2D` "/Engine/VREditor/Sounds/UI/Dockable_Window_Open.Dockable_Window_Open" 1.0 1.0 0.0 null null))))))))))

(event `self.ReceiveBeginPlay`
  ;[1 1 1] Widget
  (bind _returnvalue (`|CreateWidget` "/Game/FirstPerson/Blueprints/Interact_Wid.Interact_Wid_C"))
  (set `self.InteractPrompt` _returnvalue))

(event `self.Box.OnComponentBeginOverlap`
  (params (OverlappedComponent :type "PrimitiveComponent Object Reference") (OtherActor :type "Actor Object Reference") (OtherComp :type "PrimitiveComponent Object Reference") (OtherBodyIndex :type Integer) (bFromSweep :type Boolean) (SweepResult :type "HitResult Structure (by ref)"))
  ;[1 1 1] Widget
  (if (== OtherActor (`GameplayStatics.GetPlayerCharacter` 0))
    (`UserWidget.AddToViewport` (`self.InteractPrompt`) 0)))

(event `self.Box.OnComponentEndOverlap`
  (params (OverlappedComponent :type "PrimitiveComponent Object Reference") (OtherActor :type "Actor Object Reference") (OtherComp :type "PrimitiveComponent Object Reference") (OtherBodyIndex :type Integer))
  ;[1 1 1] Widget
  (if (== (`GameplayStatics.GetPlayerCharacter` 0) OtherActor)
    (`Widget.RemoveFromParent` (`self.InteractPrompt`))))

(fn `UserConstructionScript`)