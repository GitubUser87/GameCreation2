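; BP_SpawnEnemy_Child_Child is a main-level enemy spawner variant that places one BP_Enemy when the player enters its trigger.
; The Trigger overlap filters for BP_FirstPersonCharacter and passes through a DoOnce, so it fires only the first time.
; The enemy spawns with a fixed rotation at SpawnPoint2, converted from actor-local to world space.
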(event `self.Trigger.OnComponentBeginOverlap`
  (params (OverlappedComponent :type "PrimitiveComponent Object Reference") (OtherActor :type "Actor Object Reference") (OtherComp :type "PrimitiveComponent Object Reference") (OtherBodyIndex :type Integer) (bFromSweep :type Boolean) (SweepResult :type "HitResult Structure (by ref)"))
  (cast `/Game/FirstPerson/Blueprints/BP_FirstPersonCharacter` OtherActor)
  (`/Engine/EditorBlueprintResources/StandardMacros.DoOnce` false
    (:`Completed`
      (`AIBlueprintHelperLibrary.SpawnAIFromClass` "/Game/Maps/General_Content/Blueprints/BP_Enemy.BP_Enemy_C" null (`KismetMathLibrary.TransformLocation` (`self.GetTransform`) (`self.SpawnPoint2`)) (struct :`Yaw` 180.0) false null))))

(fn `UserConstructionScript`
  (`parent.UserConstructionScript`))