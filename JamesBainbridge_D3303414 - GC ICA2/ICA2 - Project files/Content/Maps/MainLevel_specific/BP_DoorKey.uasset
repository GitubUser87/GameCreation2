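; BP_DoorKey is a keycard-locked door that shows an interact prompt while the player is inside its Box trigger.
; Interact checks HasKey on BP_FirstPersonCharacter and, if set, plays the Open_Door timeline to lerp the Door downward from its origin.
; Without the key, it prints a message to find the keycard after a short retriggerable delay.
; The Interact_Wid prompt is created at BeginPlay and added or removed on overlap.
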(event `/Game/Maps/General_Content/Blueprints/BP_Interact_Interface.Interact`
  ;[1 1 1] This will check to see if the player has the key, if they do then it will open the door.
  (bind _asbp_first_person_character (cast `/Game/FirstPerson/Blueprints/BP_FirstPersonCharacter` (`GameplayStatics.GetPlayerCharacter` 0)))
  (if (`/Game/FirstPerson/Blueprints/BP_FirstPersonCharacter.Has Key?` _asbp_first_person_character)
    (bind (_direction _open_track) (`Timeline|Open_Door` :!via `PlayFromStart`)
      (:`Update`
        (`SceneComponent.K2_SetRelativeLocation` (`self.Door`) (`KismetMathLibrary.VLerp` (0.0 0.0 0.0) (0.0 0.0 -340.0) _open_track) false false)))
    (else
      (`KismetSystemLibrary.RetriggerableDelay` 0.5)
      (`KismetSystemLibrary.PrintString` "Please go and find the keycard to open this door."))))

(event `self.ReceiveBeginPlay`
  ;[1 1 1] Widget
  (bind _returnvalue (`|CreateWidget` "/Game/FirstPerson/Blueprints/Interact_Wid.Interact_Wid_C"))
  (set `self.Interact Prompt` _returnvalue))

(event `self.Box.OnComponentBeginOverlap`
  (params (OverlappedComponent :type "PrimitiveComponent Object Reference") (OtherActor :type "Actor Object Reference") (OtherComp :type "PrimitiveComponent Object Reference") (OtherBodyIndex :type Integer) (bFromSweep :type Boolean) (SweepResult :type "HitResult Structure (by ref)"))
  ;[1 1 1] Widget
  (if (== OtherActor (`GameplayStatics.GetPlayerCharacter` 0))
    (`UserWidget.AddToViewport` (`self.Interact Prompt`) 0)))

(event `self.Box.OnComponentEndOverlap`
  (params (OverlappedComponent :type "PrimitiveComponent Object Reference") (OtherActor :type "Actor Object Reference") (OtherComp :type "PrimitiveComponent Object Reference") (OtherBodyIndex :type Integer))
  ;[1 1 1] Widget
  (if (== (`GameplayStatics.GetPlayerCharacter` 0) OtherActor)
    (`Widget.RemoveFromParent` (`self.Interact Prompt`))))

(fn `UserConstructionScript`)