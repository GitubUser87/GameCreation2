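; Smasher hazard for the final boss map that slams at random intervals and ends the game if it hits the player.
; A random Delay on Tick paces each cycle, briefly enabling the Warning volume's pawn overlap to show a warning widget before the Crusher timeline moves the Cube.
; Player overlap with the Damage volume opens the Game Over widget, switches to UI-only input and pauses the game.
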(event `self.ReceiveTick`
  (params (DeltaSeconds :type "Float (single-precision)"))
  ;[1 1 1] Slam and warning trigger.
  (`KismetSystemLibrary.Delay` (`KismetMathLibrary.RandomFloatInRange` 3.0 10.0))
  (`|ExecutionSequence`
    (:`then_0`
      (`PrimitiveComponent.SetCollisionResponseToChannel` (`self.Warning`) "ECC_Pawn" "ECR_Overlap")
      (`KismetSystemLibrary.RetriggerableDelay` 1.0)
      (`PrimitiveComponent.SetCollisionResponseToChannel` (`self.Warning`) "ECC_Pawn" "ECR_Ignore"))
    (:`then_1`
      (`KismetSystemLibrary.Delay` 1.0)
      (bind (_direction _smash_track) (`Timeline|Crusher` :!via `PlayFromStart`)
        (:`Update`
          (`SceneComponent.K2_SetRelativeLocation` (`self.Cube`) (`KismetMathLibrary.VLerp` (0.0 0.0 -225.0) (`self.New Location`) _smash_track) false false))))))

(event `self.Damage.OnComponentBeginOverlap`
  (params (OverlappedComponent :type "PrimitiveComponent Object Reference") (OtherActor :type "Actor Object Reference") (OtherComp :type "PrimitiveComponent Object Reference") (OtherBodyIndex :type Integer) (bFromSweep :type Boolean) (SweepResult :type "HitResult Structure (by ref)"))
  (bind _returnvalue (`GameplayStatics.GetPlayerController` 0))
  ;[1 1 1] Kill
  (cast `/Game/FirstPerson/Blueprints/BP_FirstPersonCharacter` OtherActor)
  (bind _returnvalue_2 (`|CreateWidget` "/Game/FirstPerson/Blueprints/GameOver_Wid.GameOver_Wid_C"))
  (`UserWidget.AddToViewport` _returnvalue_2 0)
  (set `PlayerController.bShowMouseCursor` true _returnvalue)
  (`WidgetBlueprintLibrary.SetInputMode_UIOnlyEx` _returnvalue _returnvalue_2)
  (`GameplayStatics.SetGamePaused` true))

(event `self.Warning.OnComponentBeginOverlap`
  (params (OverlappedComponent :type "PrimitiveComponent Object Reference") (OtherActor :type "Actor Object Reference") (OtherComp :type "PrimitiveComponent Object Reference") (OtherBodyIndex :type Integer) (bFromSweep :type Boolean) (SweepResult :type "HitResult Structure (by ref)"))
  ;[1 1 1] WARNING
  (cast `/Game/FirstPerson/Blueprints/BP_FirstPersonCharacter` OtherActor)
  (bind _returnvalue (`|CreateWidget` "/Game/FirstPerson/Blueprints/Warning_Wid.Warning_Wid_C" (`GameplayStatics.GetPlayerController` 0)))
  (`UserWidget.AddToViewport` _returnvalue 0))

(event `self.Warning.OnComponentEndOverlap`
  (params (OverlappedComponent :type "PrimitiveComponent Object Reference") (OtherActor :type "Actor Object Reference") (OtherComp :type "PrimitiveComponent Object Reference") (OtherBodyIndex :type Integer))
  ;[1 1 1] WARNING
  (cast `/Game/FirstPerson/Blueprints/BP_FirstPersonCharacter` OtherActor)
  (`Widget.RemoveFromParent` (stale `self.Warning.OnComponentBeginOverlap` _returnvalue)))

(fn `UserConstructionScript`)