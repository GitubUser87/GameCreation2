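; BP_Boss is the final boss actor, which the player defeats by hitting it with first-person projectiles.
; Tick swaps the face between three random materials about once a second.
; While the player is inside its sphere trigger, a looping timer smoothly yaws the boss toward them.
; At zero health it adds score, hides itself, then after a delay shows the win widget and pauses the game.
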(event `self.ReceiveTick`
  (params (DeltaSeconds :type "Float (single-precision)"))
  ;[1 1 1] Faces
  (`KismetSystemLibrary.Delay` 1.0)
  (`PrimitiveComponent.SetMaterial` (`self.Face`) 0 (`|GetArrayItem` (`|MakeArray` "/Game/Maps/General_Content/Face1_Mat.Face1_Mat" "/Game/Maps/General_Content/Face2_Mat.Face2_Mat" "/Game/Maps/General_Content/Face3_Mat.Face3_Mat" :!type "MaterialInterface Object Reference") (`KismetMathLibrary.RandomIntegerInRange` 0 2))))

(event `self.Sphere.OnComponentBeginOverlap`
  (params (OverlappedComponent :type "PrimitiveComponent Object Reference") (OtherActor :type "Actor Object Reference") (OtherComp :type "PrimitiveComponent Object Reference") (OtherBodyIndex :type Integer) (bFromSweep :type Boolean) (SweepResult :type "HitResult Structure (by ref)"))
  ;[1 1 1] Always face player, so the player can see their target.
  (bind _asbp_first_person_character (cast `/Game/FirstPerson/Blueprints/BP_FirstPersonCharacter` OtherActor))
  (set `self.Player REF` _asbp_first_person_character)
  (bind _returnvalue (`KismetSystemLibrary.K2_SetTimerDelegate` (delegate `Rotate`) 0.01 true))
  (set `self.Timer` _returnvalue))

(event `Rotate`
  (bind (_returnvalue_roll _returnvalue_pitch _returnvalue_yaw) (`KismetMathLibrary.BreakRotator` (`KismetMathLibrary.RInterpTo` (`self.K2_GetActorRotation`) (`KismetMathLibrary.FindLookAtRotation` (`self.K2_GetActorLocation`) (`self.K2_GetActorLocation` (`self.Player REF`))) (`GameplayStatics.GetWorldDeltaSeconds`) 1.0)))
  ;[1 1 1] Always face player, so the player can see their target.
  (`self.K2_SetActorRotation` (`KismetMathLibrary.MakeRotator` 0.0 0.0 _returnvalue_yaw)))

(event `self.Sphere.OnComponentEndOverlap`
  (params (OverlappedComponent :type "PrimitiveComponent Object Reference") (OtherActor :type "Actor Object Reference") (OtherComp :type "PrimitiveComponent Object Reference") (OtherBodyIndex :type Integer))
  ;[1 1 1] Always face player, so the player can see their target.
  (`KismetSystemLibrary.K2_ClearAndInvalidateTimerHandle` (`self.Timer`)))

(event `self.Boss.OnComponentHit`
  (params (HitComponent :type "PrimitiveComponent Object Reference") (OtherActor :type "Actor Object Reference") (OtherComp :type "PrimitiveComponent Object Reference") (NormalImpulse :type "Vector Structure") (Hit :type "HitResult Structure (by ref)"))
  (bind _returnvalue (`GameplayStatics.GetPlayerController` 0))
  ;[1 1 1] Health/Win
  (cast `/Game/FirstPerson/Blueprints/BP_FirstPersonProjectile` OtherActor)
  (bind _result (`/Engine/EditorBlueprintResources/StandardMacros.DecrementInt` (`self.Health`))
    (:`  `
      (set `self.Health` _result)
      (if (== (`self.Health`) 0)
        (`|ExecutionSequence`
          (:`then_0`
            (bind _asbp_first_person_character (cast `/Game/FirstPerson/Blueprints/BP_FirstPersonCharacter` (`GameplayStatics.GetPlayerCharacter` 0)))
            (set `/Game/FirstPerson/Blueprints/BP_FirstPersonCharacter.Score` (+ (`/Game/FirstPerson/Blueprints/BP_FirstPersonCharacter.Score` _asbp_first_person_character) 200) _asbp_first_person_character)
            (`SceneComponent.SetVisibility` (`self.Boss`) false false)
            (`SceneComponent.SetVisibility` (`self.Face`) false false))
          (:`then_1`
            (`KismetSystemLibrary.Delay` 3.0)
            (bind _returnvalue_2 (`|CreateWidget` "/Game/Maps/FinalBoss_Specific/Win_Wid.Win_Wid_C" _returnvalue))
            (`UserWidget.AddToViewport` _returnvalue_2 0)
            (set `PlayerController.bShowMouseCursor` true _returnvalue)
            (`WidgetBlueprintLibrary.SetInputMode_UIOnlyEx` _returnvalue _returnvalue_2)
            (`GameplayStatics.SetGamePaused` true)))))))

(fn `UserConstructionScript`)